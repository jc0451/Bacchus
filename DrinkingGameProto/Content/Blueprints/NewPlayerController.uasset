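; Player controller for a turn-based party card game, swapping full-screen widgets for player setup, topic picking and card display.
; NextTurnEvent rotates players, offering three random distinct topics when a player's three-card allowance resets.
; GetCardInTopic draws from Cards_Table, avoiding recent repeats and occasionally substituting a Wild card, never consecutively or right after topic selection.
; It also handles lobby hosting and mirrors GameStateBacchus's multiplayer name list each tick.
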(event Custom|SinglePlayer_Event
  (Viewport|RemoveAllWidgets)
  (bind _returnvalue (UserInterface|CreateWidget "/Game/Blueprints/PlayersScreen.PlayersScreen_C"))
  (UserInterface|Viewport|AddtoViewport _returnvalue 0))

(event Custom|PlayerConfirmEvent
  (bind _foundwidgets (Widget|GetAllWidgetsOfClass "/Game/Blueprints/PlayersScreen.PlayersScreen_C" false))
  (Variables|Default|SetP_PlayersName (Variables|/Game/Blueprints/PlayersScreen.PlayersScreen_C|GetPlayerName (Utilities|Array|Get(acopy) _foundwidgets)))
  (CallFunction|NextTurnEvent))

(event Custom|PickCardsEvent
  (bind _playerturnindex (Variables|Default|GetPlayerTurnIndex))
  (bind _p_topicid (Variables|Default|GetP_TopicID))
  (bind _output (Utilities|Array|Get(acopy) _p_topicid _playerturnindex))
  (Math|Integer|DecrementInt (Utilities|Array|Get(acopy) (Variables|Default|GetP_TurnsLeft) (Variables|Default|GetPlayerTurnIndex))
    (:%20%20
      (bind (_cardgiven _topicbackground) (CallFunction|GetCardinTopic (Utilities|Array|Get(acopy) (Variables|Default|GetTopics_Lengths) _output) _output))
      (Variables|Default|SetCard_Given _cardgiven)
      (Variables|Default|SetBack_Given _topicbackground)
      (Viewport|RemoveAllWidgets)
      (bind _returnvalue (UserInterface|CreateWidget "/Game/Blueprints/CardScreen.CardScreen_C" (Game|GetPlayerController 0)))
      (UserInterface|Viewport|AddtoViewport _returnvalue 0))))

(event Custom|NextTurnEvent
  (if (Variables|Default|GetFirstTime)
    (Variables|Default|SetFirstTime false)
    (else
      (if (> (Utilities|Array|Get(acopy) (Variables|Default|GetP_TurnsLeft) (Variables|Default|GetPlayerTurnIndex)) 0)
        _
        (else
          (Utilities|Array|SetArrayElem (Variables|Default|GetP_TurnsLeft) (Variables|Default|GetPlayerTurnIndex) 3)))
      (if (< (Variables|Default|GetPlayerTurnIndex) (- (Utilities|Array|Length (Variables|Default|GetP_PlayersName)) 1))
        (Math|Integer|IncrementInt (Variables|Default|GetPlayerTurnIndex)
          (:%20%20
            _))
        (else
          (Variables|Default|SetPlayerTurnIndex 0)))))
  (if (== (Utilities|Array|Get(acopy) (Variables|Default|GetP_TurnsLeft) (Variables|Default|GetPlayerTurnIndex)) 3)
    (CallFunction|PickTopicsEvent)
    (Variables|Default|SetWild_Last true)
    (else
      (CallFunction|PickCardsEvent))))

(event Custom|PickTopicsEvent
  (Viewport|RemoveAllWidgets)
  (bind _topics_presented (CallFunction|GenerateTopicSelection))
  (Variables|Default|SetTopic1ID (Utilities|Array|Get(acopy) _topics_presented))
  (Variables|Default|SetTopic1 (Utilities|Array|Get(acopy) (Variables|Default|GetTopics_Array) (Utilities|Array|Get(acopy) _topics_presented)))
  (Variables|Default|SetTopic2ID (Utilities|Array|Get(acopy) _topics_presented 1))
  (Variables|Default|SetTopic2 (Utilities|Array|Get(acopy) (Variables|Default|GetTopics_Array) (Utilities|Array|Get(acopy) _topics_presented 1)))
  (Variables|Default|SetTopic3ID (Utilities|Array|Get(acopy) _topics_presented 2))
  (Variables|Default|SetTopic3 (Utilities|Array|Get(acopy) (Variables|Default|GetTopics_Array) (Utilities|Array|Get(acopy) _topics_presented 2)))
  (Utilities|Array|Clear (Variables|Default|GetGenerate_Return))
  (bind _returnvalue (UserInterface|CreateWidget "/Game/Blueprints/PickTopic.PickTopic_C" (Game|GetPlayerController 0)))
  (UserInterface|Viewport|AddtoViewport _returnvalue 0))

(event Custom|MultiPlayerEvent
  (Viewport|RemoveAllWidgets)
  (bind _returnvalue (UserInterface|CreateWidget "/Game/Blueprints/MultiplayerWidget.MultiplayerWidget_C"))
  (UserInterface|Viewport|AddtoViewport _returnvalue 0))

(event Custom|PlayerHost
  (bind _asgame_instance_bp (Utilities|Casting|CastToGameInstanceBP (Game|GetGameInstance)))
  (Default|InstanceHostLobby _asgame_instance_bp self))

(event Custom|UpdateList
  (params (Name :type String))
  (bind _returnvalue (Actor|GetActorOfClass "/Game/Blueprints/GameStateBacchus.GameStateBacchus_C"))
  (Default|AddPlayerName _returnvalue Name)
  (Development|PrintString "player"))

(event Custom|Tick
  (bind _returnvalue (Actor|GetActorOfClass "/Game/Blueprints/GameStateBacchus.GameStateBacchus_C"))
  (Variables|Default|SetMP_NameList (Variables|/Game/Blueprints/GameStateBacchus.GameStateBacchus_C|GetPlayerNameList _returnvalue)))

(event EventBeginPlay
  (Utilities|FlowControl|Sequence
    (:then_0
      (Class|KismetSystemLibrary|ControlScreensaver false))
    (:then_1
      (EventDispatchers|BindEventtoPlayerConfirm (delegate Custom|PlayerConfirmEvent)))
    (:then_2
      (EventDispatchers|BindEventtoPickCards (delegate Custom|PickCardsEvent)))
    (:then_3
      (EventDispatchers|BindEventtoNextTurn (delegate Custom|NextTurnEvent)))
    (:then_4
      (EventDispatchers|BindEventtoPickTopics (delegate Custom|PickTopicsEvent)))
    (:then_5
      (EventDispatchers|BindEventtoSinglePlayer (delegate Custom|SinglePlayer_Event)))
    (:then_6
      (EventDispatchers|BindEventtoMultiPlayer (delegate Custom|MultiPlayerEvent)))
    (:then_7
      (Utilities|FlowControl|Sequence))))

(event Collision|EventActorBeginOverlap
  (params (OtherActor :type Actor%20Object%20Reference)))

(event EventTick
  (params (DeltaSeconds :type Float%20%28single-precision%29)))

(event EventEndPlay
  (params (EndPlayReason :type EEndPlayReason%20Enum :default "Destroyed"))
  (Viewport|RemoveAllWidgets))

(event Input|KeyboardEvents|AnyKey
  (params (Key :type Key%20Structure :default "None")))

(fn ConstructionScript)

(fn GenerateTopicSelection
  (for _index (range 0 2)
    (switch int _index
      (:0
        (bind _randint (CallFunction|Rand 14 1))
        (bind _output_get (Variables|Default|SetGenerate_Var _randint))
        (bind _output_get_2 (Variables|Default|SetGenerate_NoRepeat_1 _output_get))
        (Utilities|Array|Add (Variables|Default|GetGenerate_Return) _output_get_2))
      (:1
        (bind _randint_2 (CallFunction|Rand 14 1 :!label _label))
        (bind _output_get_3 (Variables|Default|SetGenerate_Var _randint_2))
        (if (!= _output_get_3 (Variables|Default|GetGenerate_NoRepeat_1))
          (bind _output_get_4 (Variables|Default|SetGenerate_NoRepeat_2 _output_get_3))
          (Utilities|Array|Add (Variables|Default|GetGenerate_Return) _output_get_4)
          (else
            (goto _label))))
      (:2
        (bind _randint_3 (CallFunction|Rand 14 1 :!label _label_2))
        (bind _output_get_5 (Variables|Default|SetGenerate_Var _randint_3))
        (if (!= _output_get_5 (Variables|Default|GetGenerate_NoRepeat_1))
          (if (!= _output_get_5 (Variables|Default|GetGenerate_NoRepeat_2))
            (bind _output_get_6 (Variables|Default|SetGenerate_NoRepeat_2 _output_get_5))
            (Utilities|Array|Add (Variables|Default|GetGenerate_Return) _output_get_6)
            (else
              (goto _label_2)))
          (else
            (goto _label_2))))))
  (return (Variables|Default|GetGenerate_Return)))

(fn GetCardinTopic
  (params (TopicRange_P :type Integer) (ID_P :type Integer))
  (Utilities|FlowControl|Sequence
    (:then_0
      (switch int ID_P
        (:1
          (Variables|Default|SetCards_Played (Variables|Default|GetPlayed_1)))
        (:2
          (Variables|Default|SetCards_Played (Variables|Default|GetPlayed_2)))
        (:3
          (Variables|Default|SetCards_Played (Variables|Default|GetPlayed_3)))
        (:4
          (Variables|Default|SetCards_Played (Variables|Default|GetPlayed_4)))
        (:5
          (Variables|Default|SetCards_Played (Variables|Default|GetPlayed_5)))
        (:6
          (Variables|Default|SetCards_Played (Variables|Default|GetPlayed_6)))
        (:7
          (Variables|Default|SetCards_Played (Variables|Default|GetPlayed_7)))
        (:8
          (Variables|Default|SetCards_Played (Variables|Default|GetPlayed_8)))
        (:9
          (Variables|Default|SetCards_Played (Variables|Default|GetPlayed_9)))
        (:10
          (Variables|Default|SetCards_Played (Variables|Default|GetPlayed_10)))
        (:11
          (Variables|Default|SetCards_Played (Variables|Default|GetPlayed_11)))
        (:12
          (Variables|Default|SetCards_Played (Variables|Default|GetPlayed_12)))
        (:13
          (Variables|Default|SetCards_Played (Variables|Default|GetPlayed_13)))
        (:14
          (Variables|Default|SetCards_Played (Variables|Default|GetPlayed_14)))))
    (:then_1
      (if (Variables|Default|GetWild_Last)
        (Variables|Default|SetWild_Last false)
        (else
          (bind _randint (CallFunction|Rand 7 1))
          (if (== _randint 7)
            (bind _randint_2 (CallFunction|Rand 48 1))
            (Variables|Default|SetWild_Last true)
            (bind _returnvalue (Utilities|GetDataTableRow "/Game/Blueprints/Cards_Table.Cards_Table" (Utilities|String|StringToName (Utilities|String|ToString(Integer) _randint_2)))
              (:then
                (return (.Wild (Utilities|Struct|BreakCardsStruct _returnvalue)) (Utilities|Array|Get(acopy) (Variables|Default|GetTopic_Backs) 15))))
            (else
              _))))
      (bind _randint_3 (CallFunction|Rand TopicRange_P 1 :!label _label))
      (if (not (Utilities|Array|ContainsItem (Variables|Default|GetCards_Played) (+ (Math|Float|Truncate (* ID_P 1e+02)) _randint_3)))
        (Utilities|Array|Add (Variables|Default|GetCards_Played) (+ (Math|Float|Truncate (* ID_P 1e+02)) _randint_3))
        (if (>= (Utilities|Array|Length (Variables|Default|GetCards_Played)) 10)
          (Utilities|Array|Clear (Variables|Default|GetCards_Played)))
        (switch int ID_P
          (:1
            (Variables|Default|SetPlayed_1 (Variables|Default|GetCards_Played)))
          (:2
            (Variables|Default|SetPlayed_2 (Variables|Default|GetCards_Played)))
          (:3
            (Variables|Default|SetPlayed_3 (Variables|Default|GetCards_Played)))
          (:4
            (Variables|Default|SetPlayed_4 (Variables|Default|GetCards_Played)))
          (:5
            (Variables|Default|SetPlayed_5 (Variables|Default|GetCards_Played)))
          (:6
            (Variables|Default|SetPlayed_6 (Variables|Default|GetCards_Played)))
          (:7
            (Variables|Default|SetPlayed_7 (Variables|Default|GetCards_Played)))
          (:8
            (Variables|Default|SetPlayed_8 (Variables|Default|GetCards_Played)))
          (:9
            (Variables|Default|SetPlayed_9 (Variables|Default|GetCards_Played)))
          (:10
            (Variables|Default|SetPlayed_10 (Variables|Default|GetCards_Played)))
          (:11
            (Variables|Default|SetPlayed_11 (Variables|Default|GetCards_Played)))
          (:12
            (Variables|Default|SetPlayed_12 (Variables|Default|GetCards_Played)))
          (:13
            (Variables|Default|SetPlayed_13 (Variables|Default|GetCards_Played)))
          (:14
            (Variables|Default|SetPlayed_14 (Variables|Default|GetCards_Played))))
        (bind _returnvalue_2 (Utilities|GetDataTableRow "/Game/Blueprints/Cards_Table.Cards_Table" (Utilities|String|StringToName (Utilities|String|ToString(Integer) _randint_3)))
          (:then
            (switch int ID_P
              (:1
                (Variables|Default|SetCard_Given (.TV (Utilities|Struct|BreakCardsStruct _returnvalue_2))))
              (:2
                (Variables|Default|SetCard_Given (.Danger (Utilities|Struct|BreakCardsStruct _returnvalue_2))))
              (:3
                (Variables|Default|SetCard_Given (.Money (Utilities|Struct|BreakCardsStruct _returnvalue_2))))
              (:4
                (Variables|Default|SetCard_Given (.Social (Utilities|Struct|BreakCardsStruct _returnvalue_2))))
              (:5
                (Variables|Default|SetCard_Given (.Wacky (Utilities|Struct|BreakCardsStruct _returnvalue_2))))
              (:6
                (Variables|Default|SetCard_Given (.Animal (Utilities|Struct|BreakCardsStruct _returnvalue_2))))
              (:7
                (Variables|Default|SetCard_Given (.Music (Utilities|Struct|BreakCardsStruct _returnvalue_2))))
              (:8
                (Variables|Default|SetCard_Given (.Personal (Utilities|Struct|BreakCardsStruct _returnvalue_2))))
              (:9
                (Variables|Default|SetCard_Given (.FoodDrinks (Utilities|Struct|BreakCardsStruct _returnvalue_2))))
              (:10
                (Variables|Default|SetCard_Given (.World (Utilities|Struct|BreakCardsStruct _returnvalue_2))))
              (:11
                (Variables|Default|SetCard_Given (.Sexy (Utilities|Struct|BreakCardsStruct _returnvalue_2))))
              (:12
                (Variables|Default|SetCard_Given (.Pop (Utilities|Struct|BreakCardsStruct _returnvalue_2))))
              (:13
                (Variables|Default|SetCard_Given (.Tech (Utilities|Struct|BreakCardsStruct _returnvalue_2))))
              (:14
                (Variables|Default|SetCard_Given (.Relationships (Utilities|Struct|BreakCardsStruct _returnvalue_2)))))
            (return (Variables|Default|GetCard_Given) (Utilities|Array|Get(acopy) (Variables|Default|GetTopic_Backs) ID_P))))
        (else
          (goto _label))))))

(fn Rand
  (params (Range_R :type Integer) (min_R :type Integer))
  (return (Math|Random|RandomIntegerinRange min_R Range_R)))