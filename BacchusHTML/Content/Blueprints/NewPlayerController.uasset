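; Player controller that runs a turn-based party card game, swapping UMG screens through bound events.
; NextTurn rotates players, offers three random topics whenever a player's three-card allowance refills, and periodically gives the score leader a Bacchus blessing, then resets scores.
; PickCards draws from standard or online DataTables by topic, looking up points, avoiding recent repeats via per-topic played lists and occasionally substituting Wild cards.
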(event Custom|SinglePlayer_Event
  (Viewport|RemoveAllWidgets)
  (bind _returnvalue (UserInterface|CreateWidget "/Game/Blueprints/PlayerScreen.PlayerScreen_C"))
  (UserInterface|Viewport|AddtoViewport _returnvalue 0))

(event Custom|PlayerConfirmEvent
  (bind _foundwidgets (Widget|GetAllWidgetsOfClass "/Game/Blueprints/PlayerScreen.PlayerScreen_C" false))
  (bind _asplayer_screen (Utilities|Casting|CastToPlayerScreen (Utilities|Array|Get(acopy) _foundwidgets)))
  (Variables|Default|SetP_PlayersName (Variables|/Game/Blueprints/PlayerScreen.PlayerScreen_C|GetPlayerName _asplayer_screen))
  (Variables|Default|SetOnline_Mode (Variables|/Game/Blueprints/PlayerScreen.PlayerScreen_C|GetOnline _asplayer_screen))
  (Variables|Default|SetTurns_Left_UI (+ (* (Utilities|Array|Length (Variables|/Game/Blueprints/PlayerScreen.PlayerScreen_C|GetPlayerName _asplayer_screen)) 3) 1))
  (Viewport|RemoveAllWidgets)
  (bind _returnvalue (UserInterface|CreateWidget "/Game/Blueprints/Tutorial.Tutorial_C"))
  (UserInterface|Viewport|AddtoViewport _returnvalue 0))

(event Custom|PickCardsEvent
  (bind _playerturnindex (Variables|Default|GetPlayerTurnIndex))
  (bind _p_topicid (Variables|Default|GetP_TopicID))
  (bind _output (Utilities|Array|Get(acopy) _p_topicid _playerturnindex))
  (if (== (Variables|Default|GetTurns_Left_UI) 1)
    (Variables|Default|SetTurns_Left_UI (* (Utilities|Array|Length (Variables|Default|GetP_PlayersName)) 3))
    (else
      (Math|Integer|DecrementInt (Variables|Default|GetTurns_Left_UI)
        (:%20%20
          _))))
  (Math|Integer|DecrementInt (Utilities|Array|Get(acopy) (Variables|Default|GetP_TurnsLeft) (Variables|Default|GetPlayerTurnIndex))
    (:%20%20
      (if (Variables|Default|GetOnline_Mode)
        (bind (_cardgiven _topicbackground _scored _points) (CallFunction|GetCardinTopicOnline (Utilities|Array|Get(acopy) (Variables|Default|GetTopics_Lengths_Online) _output) _output))
        (Variables|Default|SetCard_Given _cardgiven)
        (Variables|Default|SetBack_Given _topicbackground)
        (Variables|Default|SetGivesScore _scored)
        (Variables|Default|SetScoreGiven _points)
        (else
          (bind (_cardgiven_2 _topicbackground_2 _scored_2 _points_2) (CallFunction|GetCardinTopic (Utilities|Array|Get(acopy) (Variables|Default|GetTopics_Lengths) _output) _output))
          (Variables|Default|SetCard_Given _cardgiven_2)
          (Variables|Default|SetBack_Given _topicbackground_2)
          (Variables|Default|SetGivesScore _scored_2)
          (Variables|Default|SetScoreGiven _points_2)))
      (Viewport|RemoveAllWidgets)
      (bind _returnvalue (UserInterface|CreateWidget "/Game/Blueprints/CardScreen.CardScreen_C" (Game|GetPlayerController 0)))
      (UserInterface|Viewport|AddtoViewport _returnvalue 0)
      (for (_array_element _array_index) (Variables|Default|GetP_Score_Index)
        (if (not (>= (Variables|Default|GetHighScoreCounter) _array_element))
          (Variables|Default|SetHighScoreCounter _array_element)
          (Variables|Default|SetWinnerIndex _array_index))))))

(event Custom|NextTurnEvent
  (bind _p_score_index (Variables|Default|GetP_Score_Index))
  (if (Variables|Default|GetFirstTime)
    (Variables|Default|SetFirstTime false)
    (else
      (if (> (Utilities|Array|Get(acopy) (Variables|Default|GetP_TurnsLeft) (Variables|Default|GetPlayerTurnIndex)) 0)
        _
        (else
          (Utilities|Array|SetArrayElem (Variables|Default|GetP_TurnsLeft) (Variables|Default|GetPlayerTurnIndex) 3)))
      (if (< (Variables|Default|GetPlayerTurnIndex) (- (Utilities|Array|Length (Variables|Default|GetP_PlayersName)) 1))
        (Math|Integer|IncrementInt (Variables|Default|GetPlayerTurnIndex)
          (:%20%20
            _))
        (else
          (Variables|Default|SetPlayerTurnIndex 0)))))
  (if (== (Utilities|Array|Get(acopy) (Variables|Default|GetP_TurnsLeft) (Variables|Default|GetPlayerTurnIndex)) 3)
    (if (>= (Variables|Default|GetBacchusCounter) (* (Utilities|Array|Length (Variables|Default|GetP_PlayersName)) 2))
      (if (== (Variables|Default|GetPlayerTurnIndex) (Variables|Default|GetWinnerIndex))
        (Default|CallBacchus)
        (for (_ _array_index) _p_score_index
          (Utilities|Array|SetArrayElem _p_score_index _array_index 0)
          (Variables|Default|SetBacchusCounter 0)
          (Variables|Default|SetHighScoreCounter 0))
        (else
          (CallFunction|PickTopicsEvent :!label _label)
          (Variables|Default|SetWild_Last true)))
      (else
        (Math|Integer|IncrementInt (Variables|Default|GetBacchusCounter)
          (:%20%20
            (goto _label)))))
    (else
      (CallFunction|PickCardsEvent))))

(event Custom|PickTopicsEvent
  (Viewport|RemoveAllWidgets)
  (bind _topics_presented (CallFunction|GenerateTopicSelection))
  (Variables|Default|SetTopic1ID (Utilities|Array|Get(acopy) _topics_presented))
  (Variables|Default|SetTopic1 (Utilities|Array|Get(acopy) (Variables|Default|GetTopics_Array) (Utilities|Array|Get(acopy) _topics_presented)))
  (Variables|Default|SetTopic2ID (Utilities|Array|Get(acopy) _topics_presented 1))
  (Variables|Default|SetTopic2 (Utilities|Array|Get(acopy) (Variables|Default|GetTopics_Array) (Utilities|Array|Get(acopy) _topics_presented 1)))
  (Variables|Default|SetTopic3ID (Utilities|Array|Get(acopy) _topics_presented 2))
  (Variables|Default|SetTopic3 (Utilities|Array|Get(acopy) (Variables|Default|GetTopics_Array) (Utilities|Array|Get(acopy) _topics_presented 2)))
  (Utilities|Array|Clear (Variables|Default|GetGenerate_Return))
  (bind _returnvalue (UserInterface|CreateWidget "/Game/Blueprints/PickTopic.PickTopic_C" (Game|GetPlayerController 0)))
  (UserInterface|Viewport|AddtoViewport _returnvalue 0))

(event Custom|BacchusEvent
  (Viewport|RemoveAllWidgets)
  (Utilities|Array|SetArrayElem (Variables|Default|GetP_TopicID) (Variables|Default|GetPlayerTurnIndex) 18 true)
  (bind _returnvalue (UserInterface|CreateWidget "/Game/Blueprints/BacchusBlessing.BacchusBlessing_C" (Game|GetPlayerController 0)))
  (UserInterface|Viewport|AddtoViewport _returnvalue 0)
  (Variables|Default|SetWinnerIndex -1))

(event EventBeginPlay
  (Utilities|FlowControl|Sequence
    (:then_0
      (Class|KismetSystemLibrary|ControlScreensaver false))
    (:then_1
      (EventDispatchers|BindEventtoPlayerConfirm (delegate Custom|PlayerConfirmEvent)))
    (:then_2
      (EventDispatchers|BindEventtoPickCards (delegate Custom|PickCardsEvent)))
    (:then_3
      (EventDispatchers|BindEventtoNextTurn (delegate Custom|NextTurnEvent)))
    (:then_4
      (EventDispatchers|BindEventtoPickTopics (delegate Custom|PickTopicsEvent)))
    (:then_5
      (EventDispatchers|BindEventtoSinglePlayer (delegate Custom|SinglePlayer_Event)))
    (:then_6
      (EventDispatchers|BindEventtoBacchus (delegate Custom|BacchusEvent)))))

(event Collision|EventActorBeginOverlap
  (params (OtherActor :type Actor%20Object%20Reference)))

(event EventTick
  (params (DeltaSeconds :type Float%20%28single-precision%29)))

(event EventEndPlay
  (params (EndPlayReason :type EEndPlayReason%20Enum :default "Destroyed"))
  (Viewport|RemoveAllWidgets))

(event Input|KeyboardEvents|AnyKey
  (params (Key :type Key%20Structure)))

(fn ConstructionScript)

(fn GenerateTopicSelection
  (for _index (range 0 2)
    (switch int _index
      (:0
        (bind _randint (CallFunction|Rand 17 1))
        (bind _output_get (Variables|Default|SetGenerate_Var _randint))
        (bind _output_get_2 (Variables|Default|SetGenerate_NoRepeat_1 _output_get))
        (Utilities|Array|Add (Variables|Default|GetGenerate_Return) _output_get_2))
      (:1
        (bind _randint_2 (CallFunction|Rand 17 1 :!label _label))
        (bind _output_get_3 (Variables|Default|SetGenerate_Var _randint_2))
        (if (!= _output_get_3 (Variables|Default|GetGenerate_NoRepeat_1))
          (bind _output_get_4 (Variables|Default|SetGenerate_NoRepeat_2 _output_get_3))
          (Utilities|Array|Add (Variables|Default|GetGenerate_Return) _output_get_4)
          (else
            (goto _label))))
      (:2
        (bind _randint_3 (CallFunction|Rand 17 1 :!label _label_2))
        (bind _output_get_5 (Variables|Default|SetGenerate_Var _randint_3))
        (if (!= _output_get_5 (Variables|Default|GetGenerate_NoRepeat_1))
          (if (!= _output_get_5 (Variables|Default|GetGenerate_NoRepeat_2))
            (bind _output_get_6 (Variables|Default|SetGenerate_NoRepeat_2 _output_get_5))
            (Utilities|Array|Add (Variables|Default|GetGenerate_Return) _output_get_6)
            (else
              (goto _label_2)))
          (else
            (goto _label_2))))))
  (return (Variables|Default|GetGenerate_Return)))

(fn GetCardinTopic
  (params (Topic%20Range :type Integer) (ID :type Integer))
  (if (== ID 18)
    (bind _randint (CallFunction|Rand Topic%20Range 1))
    (bind _returnvalue (Utilities|GetDataTableRow "/Game/Blueprints/Cards_Table_3.Cards_Table_3" (Utilities|String|StringToName (Utilities|String|ToString(Integer) _randint)))
      (:then
        (bind _output_get (Variables|Default|SetCard_Given (.Bacchus (Utilities|Struct|BreakCardsStruct _returnvalue))))
        (return _output_get (Utilities|Array|Get(acopy) (Variables|Default|GetTopic_Backs) 18) false 0)))
    (else
      (Utilities|FlowControl|Sequence
        (:then_0
          (switch int ID
            (:1
              (Variables|Default|SetCards_Played (Variables|Default|GetPlayed_1)))
            (:2
              (Variables|Default|SetCards_Played (Variables|Default|GetPlayed_2)))
            (:3
              (Variables|Default|SetCards_Played (Variables|Default|GetPlayed_3)))
            (:4
              (Variables|Default|SetCards_Played (Variables|Default|GetPlayed_4)))
            (:5
              (Variables|Default|SetCards_Played (Variables|Default|GetPlayed_5)))
            (:6
              (Variables|Default|SetCards_Played (Variables|Default|GetPlayed_6)))
            (:7
              (Variables|Default|SetCards_Played (Variables|Default|GetPlayed_7)))
            (:8
              (Variables|Default|SetCards_Played (Variables|Default|GetPlayed_8)))
            (:9
              (Variables|Default|SetCards_Played (Variables|Default|GetPlayed_9)))
            (:10
              (Variables|Default|SetCards_Played (Variables|Default|GetPlayed_10)))
            (:11
              (Variables|Default|SetCards_Played (Variables|Default|GetPlayed_11)))
            (:12
              (Variables|Default|SetCards_Played (Variables|Default|GetPlayed_12)))
            (:13
              (Variables|Default|SetCards_Played (Variables|Default|GetPlayed_13)))
            (:14
              (Variables|Default|SetCards_Played (Variables|Default|GetPlayed_14)))
            (:15
              (Variables|Default|SetCards_Played (Variables|Default|GetPlayed_15)))
            (:16
              (Variables|Default|SetCards_Played (Variables|Default|GetPlayed_16)))
            (:17
              (Variables|Default|SetCards_Played (Variables|Default|GetPlayed_17)))))
        (:then_1
          (if (Variables|Default|GetWild_Last)
            (Variables|Default|SetWild_Last false)
            (bind _randint_2 (CallFunction|Rand Topic%20Range 1 :!label _label))
            (if (not (Utilities|Array|ContainsItem (Variables|Default|GetCards_Played) (+ (Math|Float|Truncate (* ID 1e+02)) _randint_2)))
              (Utilities|Array|Add (Variables|Default|GetCards_Played) (+ (Math|Float|Truncate (* ID 1e+02)) _randint_2))
              (if (>= (Utilities|Array|Length (Variables|Default|GetCards_Played)) 10)
                (Utilities|Array|Clear (Variables|Default|GetCards_Played)))
              (switch int ID
                (:1
                  (Variables|Default|SetPlayed_1 (Variables|Default|GetCards_Played)))
                (:2
                  (Variables|Default|SetPlayed_2 (Variables|Default|GetCards_Played)))
                (:3
                  (Variables|Default|SetPlayed_3 (Variables|Default|GetCards_Played)))
                (:4
                  (Variables|Default|SetPlayed_4 (Variables|Default|GetCards_Played)))
                (:5
                  (Variables|Default|SetPlayed_5 (Variables|Default|GetCards_Played)))
                (:6
                  (Variables|Default|SetPlayed_6 (Variables|Default|GetCards_Played)))
                (:7
                  (Variables|Default|SetPlayed_7 (Variables|Default|GetCards_Played)))
                (:8
                  (Variables|Default|SetPlayed_8 (Variables|Default|GetCards_Played)))
                (:9
                  (Variables|Default|SetPlayed_9 (Variables|Default|GetCards_Played)))
                (:10
                  (Variables|Default|SetPlayed_10 (Variables|Default|GetCards_Played)))
                (:11
                  (Variables|Default|SetPlayed_11 (Variables|Default|GetCards_Played)))
                (:12
                  (Variables|Default|SetPlayed_12 (Variables|Default|GetCards_Played)))
                (:13
                  (Variables|Default|SetPlayed_13 (Variables|Default|GetCards_Played)))
                (:14
                  (Variables|Default|SetPlayed_14 (Variables|Default|GetCards_Played)))
                (:15
                  (Variables|Default|SetPlayed_15 (Variables|Default|GetCards_Played)))
                (:16
                  (Variables|Default|SetPlayed_16 (Variables|Default|GetCards_Played)))
                (:17
                  (Variables|Default|SetPlayed_17 (Variables|Default|GetCards_Played))))
              (bind _returnvalue_2 (Utilities|GetDataTableRow "/Game/Blueprints/Cards_Table_3.Cards_Table_3" (Utilities|String|StringToName (Utilities|String|ToString(Integer) _randint_2)))
                (:then
                  (bind _returnvalue_3 (Utilities|GetDataTableRow "/Game/Blueprints/PointCards_DataTable2.PointCards_DataTable2" (Utilities|String|StringToName (Utilities|String|ToString(Integer) ID)))
                    (:then
                      (if (Utilities|Array|ContainsItem (.CardID (Utilities|Struct|BreakPointCards _returnvalue_3)) _randint_2)
                        (Variables|Default|SetScoreGiven (Utilities|Array|Get(acopy) (.PointValue (Utilities|Struct|BreakPointCards _returnvalue_3)) (Utilities|Array|FindItem (.CardID (Utilities|Struct|BreakPointCards _returnvalue_3)) _randint_2)))
                        (Variables|Default|SetGivesScore true)
                        (else
                          (Variables|Default|SetScoreGiven 1)
                          (Variables|Default|SetGivesScore false)))
                      (switch int ID
                        (:1
                          (Variables|Default|SetCard_Given (.TV (Utilities|Struct|BreakCardsStruct _returnvalue_2))))
                        (:2
                          (Variables|Default|SetCard_Given (.Danger (Utilities|Struct|BreakCardsStruct _returnvalue_2))))
                        (:3
                          (Variables|Default|SetCard_Given (.Money (Utilities|Struct|BreakCardsStruct _returnvalue_2))))
                        (:4
                          (Variables|Default|SetCard_Given (.Social (Utilities|Struct|BreakCardsStruct _returnvalue_2))))
                        (:5
                          (Variables|Default|SetCard_Given (.Wacky (Utilities|Struct|BreakCardsStruct _returnvalue_2))))
                        (:6
                          (Variables|Default|SetCard_Given (.Animal (Utilities|Struct|BreakCardsStruct _returnvalue_2))))
                        (:7
                          (Variables|Default|SetCard_Given (.Music (Utilities|Struct|BreakCardsStruct _returnvalue_2))))
                        (:8
                          (Variables|Default|SetCard_Given (.Personal (Utilities|Struct|BreakCardsStruct _returnvalue_2))))
                        (:9
                          (Variables|Default|SetCard_Given (.FoodDrinks (Utilities|Struct|BreakCardsStruct _returnvalue_2))))
                        (:10
                          (Variables|Default|SetCard_Given (.World (Utilities|Struct|BreakCardsStruct _returnvalue_2))))
                        (:11
                          (Variables|Default|SetCard_Given (.Sexy (Utilities|Struct|BreakCardsStruct _returnvalue_2))))
                        (:12
                          (Variables|Default|SetCard_Given (.Pop (Utilities|Struct|BreakCardsStruct _returnvalue_2))))
                        (:13
                          (Variables|Default|SetCard_Given (.Tech (Utilities|Struct|BreakCardsStruct _returnvalue_2))))
                        (:14
                          (Variables|Default|SetCard_Given (.Relationships (Utilities|Struct|BreakCardsStruct _returnvalue_2))))
                        (:15
                          (Variables|Default|SetCard_Given (.Spooky (Utilities|Struct|BreakCardsStruct _returnvalue_2))))
                        (:16
                          (Variables|Default|SetCard_Given (.Gaming (Utilities|Struct|BreakCardsStruct _returnvalue_2))))
                        (:17
                          (Variables|Default|SetCard_Given (.SportsFitness (Utilities|Struct|BreakCardsStruct _returnvalue_2)))))
                      (return (Variables|Default|GetCard_Given) (Utilities|Array|Get(acopy) (Variables|Default|GetTopic_Backs) ID) (Variables|Default|GetGivesScore) (Variables|Default|GetScoreGiven)))
                    (:RowNotFound
                      _)))
                (:RowNotFound
                  _))
              (Development|PrintString "Errow 
Row not found")
              (else
                (goto _label)))
            (else
              (bind _randint_3 (CallFunction|Rand 5 1))
              (if (== _randint_3 1)
                (bind _randint_4 (CallFunction|Rand 47 1))
                (Variables|Default|SetWild_Last true)
                (bind _returnvalue_4 (Utilities|GetDataTableRow "/Game/Blueprints/Cards_Table_2.Cards_Table_2" (Utilities|String|StringToName (Utilities|String|ToString(Integer) _randint_4)))
                  (:then
                    (bind _returnvalue_5 (Utilities|GetDataTableRow "/Game/Blueprints/PointCards_DataTable2.PointCards_DataTable2" "19")
                      (:then
                        (if (Utilities|Array|ContainsItem (.CardID (Utilities|Struct|BreakPointCards _returnvalue_5)) _randint_4)
                          (Variables|Default|SetScoreGiven (Utilities|Array|Get(acopy) (.PointValue (Utilities|Struct|BreakPointCards _returnvalue_5)) (Utilities|Array|FindItem (.CardID (Utilities|Struct|BreakPointCards _returnvalue_5)) _randint_4)))
                          (Variables|Default|SetGivesScore true)
                          (else
                            (Variables|Default|SetScoreGiven 1)
                            (Variables|Default|SetGivesScore false)))
                        (return (.Wild (Utilities|Struct|BreakCardsStruct _returnvalue_4)) (Utilities|Array|Get(acopy) (Variables|Default|GetTopic_Backs) 19) (Variables|Default|GetGivesScore) (Variables|Default|GetScoreGiven)))
                      (:RowNotFound
                        (Development|PrintString "Errow 
Row not found")))))
                (else
                  (goto _label))))))))))

(fn Rand
  (params (Range :type Integer) (Min :type Integer))
  (return (Math|Random|RandomIntegerinRange Min Range)))

(fn GetCardinTopicOnline
  (params (Topic%20Range :type Integer) (ID :type Integer))
  (if (== ID 18)
    (bind _randint (CallFunction|Rand Topic%20Range 1))
    (bind _returnvalue (Utilities|GetDataTableRow "/Game/Blueprints/Cards_Table3.Cards_Table3" (Utilities|String|StringToName (Utilities|String|ToString(Integer) _randint)))
      (:then
        (bind _output_get (Variables|Default|SetCard_Given (.Bacchus (Utilities|Struct|BreakCardsStruct _returnvalue))))
        (return _output_get (Utilities|Array|Get(acopy) (Variables|Default|GetTopic_Backs) 18) false 0)))
    (else
      (Utilities|FlowControl|Sequence
        (:then_0
          (switch int ID
            (:1
              (Variables|Default|SetCards_Played (Variables|Default|GetPlayed_1)))
            (:2
              (Variables|Default|SetCards_Played (Variables|Default|GetPlayed_2)))
            (:3
              (Variables|Default|SetCards_Played (Variables|Default|GetPlayed_3)))
            (:4
              (Variables|Default|SetCards_Played (Variables|Default|GetPlayed_4)))
            (:5
              (Variables|Default|SetCards_Played (Variables|Default|GetPlayed_5)))
            (:6
              (Variables|Default|SetCards_Played (Variables|Default|GetPlayed_6)))
            (:7
              (Variables|Default|SetCards_Played (Variables|Default|GetPlayed_7)))
            (:8
              (Variables|Default|SetCards_Played (Variables|Default|GetPlayed_8)))
            (:9
              (Variables|Default|SetCards_Played (Variables|Default|GetPlayed_9)))
            (:10
              (Variables|Default|SetCards_Played (Variables|Default|GetPlayed_10)))
            (:11
              (Variables|Default|SetCards_Played (Variables|Default|GetPlayed_11)))
            (:12
              (Variables|Default|SetCards_Played (Variables|Default|GetPlayed_12)))
            (:13
              (Variables|Default|SetCards_Played (Variables|Default|GetPlayed_13)))
            (:14
              (Variables|Default|SetCards_Played (Variables|Default|GetPlayed_14)))
            (:15
              (Variables|Default|SetCards_Played (Variables|Default|GetPlayed_15)))
            (:16
              (Variables|Default|SetCards_Played (Variables|Default|GetPlayed_16)))
            (:17
              (Variables|Default|SetCards_Played (Variables|Default|GetPlayed_17)))))
        (:then_1
          (if (Variables|Default|GetWild_Last)
            (Variables|Default|SetWild_Last false)
            (else
              (bind _randint_2 (CallFunction|Rand 5 1))
              (if (== _randint_2 5)
                (bind _randint_3 (CallFunction|Rand 48 1))
                (Variables|Default|SetWild_Last true)
                (bind _returnvalue_2 (Utilities|GetDataTableRow "/Game/Blueprints/Cards_Table_2.Cards_Table_2" (Utilities|String|StringToName (Utilities|String|ToString(Integer) _randint_3)))
                  (:then
                    (return (.Wild (Utilities|Struct|BreakCardsStruct _returnvalue_2)) (Utilities|Array|Get(acopy) (Variables|Default|GetTopic_Backs) 19) false 0)))
                (else
                  _))))
          (bind _randint_4 (CallFunction|Rand Topic%20Range 1 :!label _label))
          (if (not (Utilities|Array|ContainsItem (Variables|Default|GetCards_Played) (+ (Math|Float|Truncate (* ID 1e+02)) _randint_4)))
            (Utilities|Array|Add (Variables|Default|GetCards_Played) (+ (Math|Float|Truncate (* ID 1e+02)) _randint_4))
            (if (>= (Utilities|Array|Length (Variables|Default|GetCards_Played)) 10)
              (Utilities|Array|Clear (Variables|Default|GetCards_Played)))
            (switch int ID
              (:1
                (Variables|Default|SetPlayed_1 (Variables|Default|GetCards_Played)))
              (:2
                (Variables|Default|SetPlayed_2 (Variables|Default|GetCards_Played)))
              (:3
                (Variables|Default|SetPlayed_3 (Variables|Default|GetCards_Played)))
              (:4
                (Variables|Default|SetPlayed_4 (Variables|Default|GetCards_Played)))
              (:5
                (Variables|Default|SetPlayed_5 (Variables|Default|GetCards_Played)))
              (:6
                (Variables|Default|SetPlayed_6 (Variables|Default|GetCards_Played)))
              (:7
                (Variables|Default|SetPlayed_7 (Variables|Default|GetCards_Played)))
              (:8
                (Variables|Default|SetPlayed_8 (Variables|Default|GetCards_Played)))
              (:9
                (Variables|Default|SetPlayed_9 (Variables|Default|GetCards_Played)))
              (:10
                (Variables|Default|SetPlayed_10 (Variables|Default|GetCards_Played)))
              (:11
                (Variables|Default|SetPlayed_11 (Variables|Default|GetCards_Played)))
              (:12
                (Variables|Default|SetPlayed_12 (Variables|Default|GetCards_Played)))
              (:13
                (Variables|Default|SetPlayed_13 (Variables|Default|GetCards_Played)))
              (:14
                (Variables|Default|SetPlayed_14 (Variables|Default|GetCards_Played)))
              (:15
                (Variables|Default|SetPlayed_15 (Variables|Default|GetCards_Played)))
              (:16
                (Variables|Default|SetPlayed_16 (Variables|Default|GetCards_Played)))
              (:17
                (Variables|Default|SetPlayed_17 (Variables|Default|GetCards_Played))))
            (bind _returnvalue_3 (Utilities|GetDataTableRow "/Game/Blueprints/Cards_Table_Online.Cards_Table_Online" (Utilities|String|StringToName (Utilities|String|ToString(Integer) _randint_4)))
              (:then
                (bind _returnvalue_4 (Utilities|GetDataTableRow "/Game/Blueprints/PointCards_DataTable_online.PointCards_DataTable_online" (Utilities|String|StringToName (Utilities|String|ToString(Integer) ID)))
                  (:then
                    (if (Utilities|Array|ContainsItem (.CardID (Utilities|Struct|BreakPointCards _returnvalue_4)) _randint_4)
                      (Variables|Default|SetScoreGiven (Utilities|Array|Get(acopy) (.PointValue (Utilities|Struct|BreakPointCards _returnvalue_4)) (Utilities|Array|FindItem (.CardID (Utilities|Struct|BreakPointCards _returnvalue_4)) _randint_4)))
                      (Variables|Default|SetGivesScore true)
                      (else
                        (Variables|Default|SetScoreGiven 1)
                        (Variables|Default|SetGivesScore false)))
                    (switch int ID
                      (:1
                        (Variables|Default|SetCard_Given (.TV (Utilities|Struct|BreakCardsStruct _returnvalue_3))))
                      (:2
                        (Variables|Default|SetCard_Given (.Danger (Utilities|Struct|BreakCardsStruct _returnvalue_3))))
                      (:3
                        (Variables|Default|SetCard_Given (.Money (Utilities|Struct|BreakCardsStruct _returnvalue_3))))
                      (:4
                        (Variables|Default|SetCard_Given (.Social (Utilities|Struct|BreakCardsStruct _returnvalue_3))))
                      (:5
                        (Variables|Default|SetCard_Given (.Wacky (Utilities|Struct|BreakCardsStruct _returnvalue_3))))
                      (:6
                        (Variables|Default|SetCard_Given (.Animal (Utilities|Struct|BreakCardsStruct _returnvalue_3))))
                      (:7
                        (Variables|Default|SetCard_Given (.Music (Utilities|Struct|BreakCardsStruct _returnvalue_3))))
                      (:8
                        (Variables|Default|SetCard_Given (.Personal (Utilities|Struct|BreakCardsStruct _returnvalue_3))))
                      (:9
                        (Variables|Default|SetCard_Given (.FoodDrinks (Utilities|Struct|BreakCardsStruct _returnvalue_3))))
                      (:10
                        (Variables|Default|SetCard_Given (.World (Utilities|Struct|BreakCardsStruct _returnvalue_3))))
                      (:11
                        (Variables|Default|SetCard_Given (.Sexy (Utilities|Struct|BreakCardsStruct _returnvalue_3))))
                      (:12
                        (Variables|Default|SetCard_Given (.Pop (Utilities|Struct|BreakCardsStruct _returnvalue_3))))
                      (:13
                        (Variables|Default|SetCard_Given (.Tech (Utilities|Struct|BreakCardsStruct _returnvalue_3))))
                      (:14
                        (Variables|Default|SetCard_Given (.Relationships (Utilities|Struct|BreakCardsStruct _returnvalue_3))))
                      (:15
                        (Variables|Default|SetCard_Given (.Spooky (Utilities|Struct|BreakCardsStruct _returnvalue_3))))
                      (:16
                        (Variables|Default|SetCard_Given (.Gaming (Utilities|Struct|BreakCardsStruct _returnvalue_3))))
                      (:17
                        (Variables|Default|SetCard_Given (.SportsFitness (Utilities|Struct|BreakCardsStruct _returnvalue_3)))))
                    (return (Variables|Default|GetCard_Given) (Utilities|Array|Get(acopy) (Variables|Default|GetTopic_Backs) ID) (Variables|Default|GetGivesScore) (Variables|Default|GetScoreGiven)))
                  (:RowNotFound
                    _)))
              (:RowNotFound
                _))
            (Development|PrintString "Errow 
Row not found")
            (else
              (goto _label))))))))